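; A master foliage spline actor, filed under Ivy, that scatters static meshes along an editable spline at construction.
; It first snaps each spline point to surfaces with visibility line traces spanning a threshold vector around the point.
; If spawning is enabled, it places collision-free, decal-free meshes at fixed spacing with a constant offset.
; Mesh, material, rotation and scale use unseeded randomness, so results change on each reconstruction.
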(fn `UserConstructionScript`
  (bind (_meshoffset_x _meshoffset_y _meshoffset_z) (`KismetMathLibrary.BreakVector` (`self.MeshOffset`)))
  (bind (_meshscale_x _meshscale_y _meshscale_z) (`KismetMathLibrary.BreakVector` (`self.MeshScale`)))
  (bind (_max_randomerotation_x _max_randomerotation_y _max_randomerotation_z) (`KismetMathLibrary.BreakVector` (`self.Max_RandomeRotation`)))
  (bind _material (`self.Material`))
  (bind _mesh (`self.Mesh`))
  (bind (_snapthreshold_x_x _snapthreshold_x_y _snapthreshold_x_z) (`KismetMathLibrary.BreakVector` (`self.SnapThreshold_X`)))
  (bind (_meshrotation_roll _meshrotation_pitch _meshrotation_yaw) (`KismetMathLibrary.BreakRotator` (`self.MeshRotation`)))
  (bind (_maxrandomescale_x _maxrandomescale_y _maxrandomescale_z) (`KismetMathLibrary.BreakVector` (`self.MaxRandomeScale`)))
  (`|ExecutionSequence`
    (:`then_0`
      ;[1 1 1] Snap Spline to Surface
      (for _index (range (`SplineComponent.GetNumberOfSplinePoints` (`self.Spline`)))
        (bind (_returnvalue_x _returnvalue_y _returnvalue_z) (`KismetMathLibrary.BreakVector` (`SplineComponent.GetLocationAtSplinePoint` (`self.Spline`) _index "World")))
        (bind (_returnvalue_x_2 _returnvalue_y_2 _returnvalue_z_2) (`KismetMathLibrary.BreakVector` (`SplineComponent.GetLocationAtSplinePoint` (`self.Spline`) _index "World")))
        (bind (_outhit _returnvalue) (`KismetSystemLibrary.LineTraceSingle` :`Start` (`KismetMathLibrary.MakeVector` (+ _snapthreshold_x_x _returnvalue_x) (+ _returnvalue_y _snapthreshold_x_y) (+ _returnvalue_z _snapthreshold_x_z)) :`End` (`KismetMathLibrary.MakeVector` (- _returnvalue_x_2 _snapthreshold_x_x) (- _returnvalue_y_2 _snapthreshold_x_y) (- _returnvalue_z_2 _snapthreshold_x_z)) :`TraceChannel` "TraceTypeQuery1" :`DrawDebugType` "ForDuration"))
        (if _returnvalue
          (`SplineComponent.SetLocationAtSplinePoint` (`self.Spline`) _index (`.Location` (`GameplayStatics.BreakHitResult` _outhit)) "World" true))))
    (:`then_1`
      (if (`self.Spawn Objects`)
        (for _index_2 (range (+ (`KismetMathLibrary.FTrunc` (/ (`SplineComponent.GetSplineLength` (`self.Spline`)) (* (`self.DistanceBetwenMeshes`) 100.0))) 1))
          (bind _returnvalue_2 (`AddComponent|NODE_AddStaticMeshComponent-0`))
          (bind (_returnvalue_x_3 _returnvalue_y_3 _returnvalue_z_3) (`KismetMathLibrary.BreakVector` (`SplineComponent.GetLocationAtDistanceAlongSpline` (`self.Spline`) (* _index_2 (* (`self.DistanceBetwenMeshes`) 100.0)) "World")))
          ;[1 1 1] fix projection
          (`SceneComponent.K2_SetWorldTransform` _returnvalue_2 (`KismetMathLibrary.MakeTransform` (`KismetMathLibrary.MakeVector` (+ _meshoffset_x _returnvalue_x_3) (+ _meshoffset_y _returnvalue_y_3) (+ _returnvalue_z_3 _meshoffset_z)) (`KismetMathLibrary.MakeRotator` (+ _meshrotation_roll (`KismetMathLibrary.RandomFloatInRange` (* _max_randomerotation_x -1.0) _max_randomerotation_x)) (+ _meshrotation_pitch (`KismetMathLibrary.RandomFloatInRange` (* _max_randomerotation_y -1.0) _max_randomerotation_y)) (+ _meshrotation_yaw (`KismetMathLibrary.RandomFloatInRange` (* _max_randomerotation_z -1.0) _max_randomerotation_z))) (`KismetMathLibrary.MakeVector` (+ _meshscale_x (`KismetMathLibrary.RandomFloatInRange` (* _maxrandomescale_x -1.0) _maxrandomescale_x)) (+ _meshscale_y (`KismetMathLibrary.RandomFloatInRange` (* _maxrandomescale_y -1.0) _maxrandomescale_y)) (+ _meshscale_z (`KismetMathLibrary.RandomFloatInRange` (* _maxrandomescale_z -1.0) _maxrandomescale_z)))) false false)
          (`StaticMeshComponent.SetStaticMesh` _returnvalue_2 (`|GetArrayItem` _mesh (`KismetMathLibrary.RandomInteger` (`KismetArrayLibrary.Array_Length` _mesh))))
          (`PrimitiveComponent.SetCollisionEnabled` _returnvalue_2 "NoCollision")
          (`PrimitiveComponent.SetMaterial` _returnvalue_2 0 (`|GetArrayItem` _material (`KismetMathLibrary.RandomInteger` (`KismetArrayLibrary.Array_Length` _material))))
          (`PrimitiveComponent.SetReceivesDecals` _returnvalue_2 false))))))