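; House switch Blueprint in the Blockout folder: a pressable button that signals the garage, with a light toggled by house power.
; Interaction, locked by an Active flag until finished, plays a timeline that moves the button and calls GarageButtonPressed on every update.
; HousePower flip-flops the point light's visibility.
; The power-switch and generator checks are disconnected, so the garage call is ungated.
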(event `HousePower`
  (`/Engine/EditorBlueprintResources/StandardMacros.FlipFlop`
    (:`A`
      (`SceneComponent.SetVisibility` (`self.PointLight`) true false))
    (:`B`
      (`SceneComponent.SetVisibility` (`self.PointLight`) false false))))

(event `/Game/FirstPersonBP/Blueprints/Interaction_Interface.Interaction`
  (params (Interactor :type "Actor Object Reference"))
  (if (not (`self.Active`))
    (set `self.Active` true)
    (bind (_direction _newtrack_0) (`Timeline|Timeline_0` :!via `PlayFromStart`)
      (:`Update`
        (`SceneComponent.K2_SetRelativeLocation` (`self.ButtonRoot`) (`KismetMathLibrary.MakeVector` 0.0 _newtrack_0) false false)
        (`/Game/Props/AdditionalProps/Doors/Garage_Button.GarageButton_Pressed` (`self.Garage`)))
      (:`Finished`
        (set `self.Active` false)))))

(fn `UserConstructionScript`)