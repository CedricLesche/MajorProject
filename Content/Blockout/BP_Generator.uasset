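; Interactable generator that the player starts with inventory items, and that shuts down on the CatchPlayerInWorkshop event.
; Interaction spends fuel to fill the tank, plus a cold-start item until the engine has run once, reporting shortages through FirstPersonGameMode.
; A successful start empties the tank, swaps the material, shows smoke and spawns an attenuated compressor sound, all reversed on shutdown except the tank.
; An InUse flag blocks overlapping interactions.
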(event `CatchPlayerInWorkshop`
  (`KismetSystemLibrary.PrintString` "Hello")
  (set `self.GeneratorIsActive` false)
  (`PrimitiveComponent.SetMaterial` (`self.Generator`) 0 "/Game/MAterials/MI_Base_Blood.MI_Base_Blood")
  (`SceneComponent.SetVisibility` (`self.PFX_Generator_Smoke`) false false)
  (`AudioComponent.Stop` (stale `/Game/FirstPersonBP/Blueprints/Interaction_Interface.Interaction` _returnvalue)))

(event `/Game/FirstPersonBP/Blueprints/Interaction_Interface.Interaction`
  (params (Interactor :type "Actor Object Reference"))
  (bind _itemcost (`self.ItemCost`))
  (if (`self.GeneratorIsActive`)
    _
    (elif (not (`self.InUse`))
      (set `self.InUse` true)
      (if (`self.TankFilled`)
        ;[1 1 1] Has the engine run before?
        (if (`self.HasbeenStartetOnce`) :!label _label
          (set `self.TankFilled` false :!label _label_2)
          (set `self.GeneratorIsActive` true)
          (`KismetSystemLibrary.PrintString` "Hello")
          (set `self.HasbeenStartetOnce` true)
          (`PrimitiveComponent.SetMaterial` (`self.Generator`) 0 "/Game/MAterials/MI_Base_Laub_2.MI_Base_Laub_2")
          (`SceneComponent.SetVisibility` (`self.PFX_Generator_Smoke`) true false)
          (bind _returnvalue (`GameplayStatics.SpawnSoundAtLocation` "/Game/Audio/Samples/A_337446_Compressor.A_337446_Compressor" (`SceneComponent.K2_GetComponentLocation` (`self.Generator`)) (struct) 1.0 1.0 0.0 "/Game/Audio/Attenuation_Generator.Attenuation_Generator" null))
          (set `self.InUse` false)
          (else
            (bind _inventory_component (`/Game/FirstPersonBP/Blueprints/FirstPersonCharacter.Inventory_Component` (stale _asfirst_person_character)))
            ;[1 1 1] Asking to Support a ColdStart
            (if (>= (`BlueprintMapLibrary.Map_Find` (`/Game/FirstPersonBP/Blueprints/Inventory_Component.CollectedItems_Map` _inventory_component) (`self.ItemNeedet_ColdStart`)) (`self.ItemCost_ColdStart`))
              (`/Game/FirstPersonBP/Blueprints/Inventory_Component.UsedAnItem` _inventory_component (`self.ItemNeedet_ColdStart`) (`self.ItemCost_ColdStart`))
              (goto _label_2)
              (else
                (`/Game/FirstPersonBP/Blueprints/FirstPersonGameMode.UsingObjectError` (stale _asfirst_person_game_mode) (`self.ErrorCode_ColdStart`) 0)
                (`KismetSystemLibrary.Delay` 2.5)
                (set `self.InUse` false)))))
        (else
          (bind _asfirst_person_character (cast `/Game/FirstPersonBP/Blueprints/FirstPersonCharacter` (`GameplayStatics.GetPlayerCharacter` 0)))
          (bind _asfirst_person_game_mode (cast `/Game/FirstPersonBP/Blueprints/FirstPersonGameMode` (`GameplayStatics.GetGameMode`)))
          ;[1 1 1] Asking For Fuel
          (if (>= (`BlueprintMapLibrary.Map_Find` (`/Game/FirstPersonBP/Blueprints/Inventory_Component.CollectedItems_Map` _inventory_component) (`self.ItemNeedetToStart`)) _itemcost)
            (`/Game/FirstPersonBP/Blueprints/Inventory_Component.UsedAnItem` _inventory_component (`self.ItemNeedetToStart`) (`self.ItemCost`))
            (set `self.TankFilled` true)
            (goto _label)
            (else
              (`/Game/FirstPersonBP/Blueprints/FirstPersonGameMode.UsingObjectError` _asfirst_person_game_mode (`self.No Fuel`) _itemcost)
              (set `self.InUse` false))))))))

(fn `UserConstructionScript`)