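; BP_PowerSwitch is a blockout switch that toggles power between a bunker and a house.
; Each Interaction event flips the Bunker and House booleans and passes House to HousePower on Schalter actors.
; Timelines drive the pitch of StaticMesh3, one played forward and the other in reverse.
; The Schalter lookup runs only when switching to House; the return branch reuses its result.
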(event `/Game/FirstPersonBP/Blueprints/Interaction_Interface.Interaction`
  (params (Interactor :type "Actor Object Reference"))
  (if (`self.Bunker`)
    (set `self.Bunker` false)
    (bind _output_get (set `self.House` true))
    (bind _outactors (`GameplayStatics.GetAllActorsOfClass` "/Game/Blockout/Schalter.Schalter_C"))
    (`/Game/Blockout/Schalter.HousePower` _outactors _output_get)
    (bind (_direction _newtrack_0) (`Timeline|Timeline_0` :!via `PlayFromStart`)
      (:`Update`
        (`SceneComponent.K2_SetRelativeRotation` (`self.StaticMesh3`) (`KismetMathLibrary.MakeRotator` 0.0 _newtrack_0) false false)))
    (else
      (bind _output_get_2 (set `self.House` false))
      (set `self.Bunker` true)
      (`/Game/Blockout/Schalter.HousePower` _outactors _output_get_2)
      (bind (_direction_2 _newtrack_0_2) (`Timeline|Timeline_1` :!via `ReverseFromEnd`)
        (:`Update`
          (`SceneComponent.K2_SetRelativeRotation` (`self.StaticMesh3`) (`KismetMathLibrary.MakeRotator` 0.0 _newtrack_0_2) false false))))))

(fn `UserConstructionScript`)