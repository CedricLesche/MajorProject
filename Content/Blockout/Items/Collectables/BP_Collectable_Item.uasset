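; BP_Collectable_Item is a blockout collectable actor that the player picks up through its Interaction event.
; On interaction, it casts player character 0 to FirstPersonCharacter and adds its ItemName to the InventoryComponent's CollectedItemsMap at zero if that key is missing.
; It then destroys itself and passes ItemName to the inventory's CollectedAnItem, leaving further collection handling to that component.
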(event `/Game/FirstPersonBP/Blueprints/Interaction_Interface.Interaction`
  (params (Interactor :type "Actor Object Reference"))
  (bind _asfirst_person_character (cast `/Game/FirstPersonBP/Blueprints/FirstPersonCharacter` (`GameplayStatics.GetPlayerCharacter` 0)))
  (bind _inventory_component (`/Game/FirstPersonBP/Blueprints/FirstPersonCharacter.Inventory_Component` _asfirst_person_character))
  (bind _collecteditems_map (`/Game/FirstPersonBP/Blueprints/Inventory_Component.CollectedItems_Map` _inventory_component))
  (if (not (`BlueprintMapLibrary.Map_Contains` _collecteditems_map (`self.ItemName`)))
    (`BlueprintMapLibrary.Map_Add` _collecteditems_map (`self.ItemName`)))
  (`self.K2_DestroyActor`)
  (`/Game/FirstPersonBP/Blueprints/Inventory_Component.CollectedAnItem` _inventory_component (`self.ItemName`)))

(fn `UserConstructionScript`)