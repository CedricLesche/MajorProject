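; Blockout water actor that moves its water vertically when DrippingWater fires and short-circuits connector boxes.
; Two chained timelines drive the water's relative Z after a brief delay.
; In a second delayed branch, the particle system moves just above the water with a spark sound.
; Until Activated is set, that branch also briefly shows the particles and calls ShortCircuite on all BP_ConectorBox actors.
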(event `DrippingWater`
  (bind (_returnvalue_x _returnvalue_y _returnvalue_z) (`KismetMathLibrary.BreakVector` (`SceneComponent.K2_GetComponentLocation` (`self.Water`))))
  (bind _returnvalue (`KismetMathLibrary.MakeVector` _returnvalue_x _returnvalue_y (+ _returnvalue_z 10.0)))
  (`|ExecutionSequence`
    (:`then_0`
      (`KismetSystemLibrary.Delay` 0.2)
      (bind (_direction _watergetup) (`Timeline|Timeline_0`)
        (:`Update`
          (`SceneComponent.K2_SetRelativeLocation` (`self.Water`) (`KismetMathLibrary.MakeVector` 0.0 0.0 _watergetup) false false))
        (:`Finished`
          (bind (_direction_2 _newtrack_0) (`Timeline|Timeline_1`)
            (:`Update`
              (`SceneComponent.K2_SetRelativeLocation` (`self.Water`) (`KismetMathLibrary.MakeVector` 0.0 0.0 _newtrack_0) false false))))))
    (:`then_1`
      (`KismetSystemLibrary.Delay` 2.0)
      (`SceneComponent.K2_SetWorldLocation` (`self.ParticleSystem`) _returnvalue false false)
      (`GameplayStatics.PlaySoundAtLocation` "/Game/Audio/Samples/ExternalSounds/A_31348_Spark.A_31348_Spark" _returnvalue (struct) 0.1 1.0 0.0 null null null)
      (if (not (`self.activated`))
        (`SceneComponent.SetVisibility` (`self.ParticleSystem`) true false)
        (bind _outactors (`GameplayStatics.GetAllActorsOfClass` "/Game/Props/Infra/Power/BP_ConectorBox.BP_ConectorBox_C"))
        (`/Game/Props/Infra/Power/BP_ConectorBox.ShortCircuite` _outactors)
        (`KismetSystemLibrary.Delay` 1.5)
        (`SceneComponent.SetVisibility` (`self.ParticleSystem`) false false)
        (set `self.activated` true)))))

(fn `UserConstructionScript`)