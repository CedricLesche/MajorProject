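; BP_Transformator is a blockout transformer whose status lights show the state of generator, solar and wind power.
; When its box trigger begins overlap, it refreshes the lights from referenced Generator, WaterTank and FuseBox states.
; The generator light mirrors whether the generator is active.
; Solar and wind lights share one state, going dark only when the water tank has been activated once and the fuse box is unrepaired.
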(event `self.Box.OnComponentBeginOverlap`
  (params (OverlappedComponent :type "PrimitiveComponent Object Reference") (OtherActor :type "Actor Object Reference") (OtherComp :type "PrimitiveComponent Object Reference") (OtherBodyIndex :type Integer) (bFromSweep :type Boolean) (SweepResult :type "HitResult Structure (by ref)"))
  (bind _generator_light (`self.Generator_Light`))
  (bind _solar_light (`self.Solar_Light`))
  (`|ExecutionSequence`
    (:`then_0`
      ;[1 1 1] Condition for Genereator_Light to change State
      (if (`/Game/Blockout/BP_Generator.GeneratorIsActive` (`self.Generator`))
        (`SceneComponent.SetVisibility` _generator_light true false)
        (else
          (`SceneComponent.SetVisibility` _generator_light false false))))
    (:`then_1`
      ;[1 1 1] Condition for Wind/Solar_Light to change State
      (if (`/Game/Props/Infra/Water/BP_Watertank_ShortCircuit.ActivatedOnce` (`self.WaterTank`))
        (if (`/Game/Blockout/FuseBox.Repaired` (`self.FuseBox`))
          (`SceneComponent.SetVisibility` _solar_light true false :!label _label)
          (`SceneComponent.SetVisibility` (`self.Wind_Light`) true false)
          (else
            (`SceneComponent.SetVisibility` _solar_light false false)
            (`SceneComponent.SetVisibility` (`self.Wind_Light`) false false)))
        (else
          (goto _label))))))

(fn `UserConstructionScript`)