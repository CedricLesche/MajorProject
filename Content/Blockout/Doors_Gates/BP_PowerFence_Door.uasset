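; Electrified fence door that can only be swung open or closed once its power has been shorted out.
; ShortCircuit_Door waits briefly, hides four particle systems and flags the power as deactivated.
; Interaction reports an error through FirstPersonGameMode while powered; otherwise it toggles the door via two timelines that yaw BladeRoot, ignoring input mid-animation.
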(event `Short Circuit_Door`
  (`KismetSystemLibrary.Delay` 0.3)
  (`SceneComponent.SetVisibility` (`self.ParticleSystem2`) false true)
  (`SceneComponent.SetVisibility` (`self.ParticleSystem3`) false true)
  (`SceneComponent.SetVisibility` (`self.ParticleSystem0`) false true)
  (`SceneComponent.SetVisibility` (`self.ParticleSystem1`) false true)
  (set `self.PowerDeactivated` true))

(event `/Game/FirstPersonBP/Blueprints/Interaction_Interface.Interaction`
  (params (Interactor :type "Actor Object Reference"))
  (bind _asfirst_person_game_mode (cast `/Game/FirstPersonBP/Blueprints/FirstPersonGameMode` (`GameplayStatics.GetGameMode`)))
  (if (`self.PowerDeactivated`)
    (if (not (`self.AnimationInProgress`))
      (set `self.AnimationInProgress` true)
      (if (`self.Door_Open`)
        (bind (_direction _doorrotation) (`Timeline|Timeline_0` :!via `PlayFromStart`)
          (:`Update`
            (`SceneComponent.K2_SetRelativeLocationAndRotation` (`self.BladeRoot`) (0.0 0.0 0.0) (`KismetMathLibrary.MakeRotator` 0.0 0.0 _doorrotation) false false)
            (set `self.Door_Open` false))
          (:`Finished`
            (set `self.AnimationInProgress` false)))
        (else
          (bind (_direction_2 _doorrotation_2) (`Timeline|Timeline_1` :!via `ReverseFromEnd`)
            (:`Update`
              (`SceneComponent.K2_SetRelativeLocationAndRotation` (`self.BladeRoot`) (0.0 0.0 0.0) (`KismetMathLibrary.MakeRotator` 0.0 0.0 _doorrotation_2) false false)
              (set `self.Door_Open` true))
            (:`Finished`
              (set `self.AnimationInProgress` false))))))
    (else
      (`/Game/FirstPersonBP/Blueprints/FirstPersonGameMode.UsingObjectError` _asfirst_person_game_mode (`self.ErrorCode`) 0))))

(fn `UserConstructionScript`)