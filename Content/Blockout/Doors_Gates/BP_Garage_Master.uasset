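; Blockout garage gate Blueprint that toggles a Cube between open and closed via an Interaction event.
; Separate timelines drive the Cube's relative location, one played forward to open and one reversed to close, while a flag blocks input during movement.
; The first opening requires an overlap with the Trigger, which does not filter actors; afterwards Interaction works regardless of overlap.
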(event `/Game/FirstPersonBP/Blueprints/Interaction_Interface.Interaction`
  (params (Interactor :type "Actor Object Reference"))
  (bind _cube (`self.Cube`))
  (if (`self.once opended`)
    (if (not (`self.AnimationInProgress`)) :!label _label
      (set `self.AnimationInProgress` true)
      (if (`self.Gate Closed`)
        (bind (_direction _newtrack_4) (`Timeline|Timeline_0` :`NewTime` 1.0 :!via `PlayFromStart`)
          (:`Update`
            (`SceneComponent.K2_SetRelativeLocation` _cube _newtrack_4 false false)
            (set `self.Gate Closed` false)
            (set `self.once opended` true))
          (:`Finished`
            (set `self.AnimationInProgress` false)))
        (else
          (bind (_direction_2 _newtrack_4_2) (`Timeline|Timeline_1` :`NewTime` 1.0 :!via `ReverseFromEnd`)
            (:`Update`
              (`SceneComponent.K2_SetRelativeLocation` _cube _newtrack_4_2 false false)
              (set `self.Gate Closed` true))
            (:`Finished`
              (set `self.AnimationInProgress` false))))))
    (elif (`self.Player is able`)
      (goto _label))))

(event `self.Trigger.OnComponentBeginOverlap`
  (params (OverlappedComponent :type "PrimitiveComponent Object Reference") (OtherActor :type "Actor Object Reference") (OtherComp :type "PrimitiveComponent Object Reference") (OtherBodyIndex :type Integer) (bFromSweep :type Boolean) (SweepResult :type "HitResult Structure (by ref)"))
  (set `self.Player is able` true))

(event `self.Trigger.OnComponentEndOverlap`
  (params (OverlappedComponent :type "PrimitiveComponent Object Reference") (OtherActor :type "Actor Object Reference") (OtherComp :type "PrimitiveComponent Object Reference") (OtherBodyIndex :type Integer))
  (set `self.Player is able` false))

(fn `UserConstructionScript`)