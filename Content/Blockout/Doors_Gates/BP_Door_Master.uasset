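; Master door/gate Blueprint that opens and closes on Interaction, gated by an item in the player's inventory.
; The item cost is charged on every use or only on the first, per CostsEveryTime; shortfalls report an error to the GameMode and play a latch sound.
; An optional destroyable mesh changes material and hides before two timelines rotate BladeRoot, with a flag blocking input mid-animation.
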(event `/Game/FirstPersonBP/Blueprints/Interaction_Interface.Interaction`
  (params (Interactor :type "Actor Object Reference"))
  (bind _itemcost (`self.ItemCost`))
  (bind _destroyablemesh (`self.DestroyableMesh`))
  (bind _asfirst_person_character (cast `/Game/FirstPersonBP/Blueprints/FirstPersonCharacter` (`GameplayStatics.GetPlayerCharacter` 0)))
  (bind _asfirst_person_game_mode (cast `/Game/FirstPersonBP/Blueprints/FirstPersonGameMode` (`GameplayStatics.GetGameMode`)))
  (if (`self.CostsEveryTime`)
    (bind _inventory_component (`/Game/FirstPersonBP/Blueprints/FirstPersonCharacter.Inventory_Component` _asfirst_person_character))
    (bind _value (`BlueprintMapLibrary.Map_Find` (`/Game/FirstPersonBP/Blueprints/Inventory_Component.CollectedItems_Map` _inventory_component) (`self.ItemNeededToOpen`)))
    (if (>= _value 1) :!label _label
      (if (>= _value _itemcost)
        (if (not (`self.AnimationInProgress`))
          (set `self.AnimationInProgress` true)
          (`/Game/FirstPersonBP/Blueprints/Inventory_Component.UsedAnItem` _inventory_component (`self.ItemNeededToOpen`) (`self.ItemCost`))
          (if (`self.DestroyableObject`)
            (`PrimitiveComponent.SetMaterial` _destroyablemesh 0 "/Game/Blockout/MAterials/MI_Base_Blood.MI_Base_Blood")
            (`KismetSystemLibrary.Delay` 0.5)
            (`SceneComponent.SetVisibility` _destroyablemesh false true)
            (`KismetSystemLibrary.Delay` 1.0))
          (set `self.OpendOnce` true)
          (if (`self.Door_Open`) :!label _label_2
            (bind (_direction _doorrotation) (`Timeline|Timeline_0` :!via `PlayFromStart`)
              (:`Update`
                (`SceneComponent.K2_SetRelativeLocationAndRotation` (`self.BladeRoot`) (0.0 0.0 0.0) (`KismetMathLibrary.MakeRotator` 0.0 0.0 _doorrotation) false false)
                (set `self.Door_Open` false))
              (:`Finished`
                (set `self.AnimationInProgress` false)))
            (else
              (bind (_direction_2 _doorrotation_2) (`Timeline|Timeline_1` :!via `ReverseFromEnd`)
                (:`Update`
                  (`SceneComponent.K2_SetRelativeLocationAndRotation` (`self.BladeRoot`) (0.0 0.0 0.0) (`KismetMathLibrary.MakeRotator` 0.0 0.0 _doorrotation_2) false false)
                  (set `self.Door_Open` true))
                (:`Finished`
                  (set `self.AnimationInProgress` false))))))
        (else
          (`/Game/FirstPersonBP/Blueprints/FirstPersonGameMode.UsingObjectError` _asfirst_person_game_mode (`self.ErrorCode`) (* (- _value _itemcost) -1) :!label _label_3)
          (`GameplayStatics.PlaySoundAtLocation` "/Game/Audio/Samples/A_126041_GateLatch.A_126041_GateLatch" (`SceneComponent.K2_GetComponentLocation` (`self.BladeRoot`)) (struct) 1.0 1.0 0.0 null null null)))
      (else
        (goto _label_3)))
    (elif (`self.OpendOnce`)
      (if (not (`self.AnimationInProgress`))
        (set `self.AnimationInProgress` true)
        (goto _label_2))
      (else
        (goto _label)))))

(fn `UserConstructionScript`)