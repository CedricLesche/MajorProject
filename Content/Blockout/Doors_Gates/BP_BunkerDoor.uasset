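; BP_BunkerDoor is a bunker door that swings open on interaction once the bunker's power and fuse requirements are met.
; The Interaction event reads the Bunker flag on the first BP_PowerSwitch found, then the Repaired flag on the first FuseBox.
; When both are true, a timeline drives BladeRoot's yaw.
; DoorOpen and AnimationInProgress are only ever set to false here, never checked.
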(event `/Game/FirstPersonBP/Blueprints/Interaction_Interface.Interaction`
  (params (Interactor :type "Actor Object Reference"))
  (bind _outactors (`GameplayStatics.GetAllActorsOfClass` "/Game/Blockout/BP_PowerSwitch.BP_PowerSwitch_C"))
  (if (`/Game/Blockout/BP_PowerSwitch.Bunker` (`|GetArrayItem` _outactors))
    (bind _outactors_2 (`GameplayStatics.GetAllActorsOfClass` "/Game/Blockout/FuseBox.FuseBox_C"))
    (if (`/Game/Blockout/FuseBox.Repaired` (`|GetArrayItem` _outactors_2))
      (bind (_direction _doorrotation) (`Timeline|Timeline_0`)
        (:`Update`
          (`SceneComponent.K2_SetRelativeLocationAndRotation` (`self.BladeRoot`) (0.0 0.0 0.0) (`KismetMathLibrary.MakeRotator` 0.0 0.0 _doorrotation) false false)
          (set `self.Door_Open` false))
        (:`Finished`
          (set `self.AnimationInProgress` false))))))

(fn `UserConstructionScript`)