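; Bunker switch that the player can trigger to operate the bunker door, with a point light toggled by power events.
; Interaction plays a timeline that moves the button along Y, with an Active flag blocking retriggers until it finishes.
; On every timeline update, it calls the door's button event if the PowerSwitch routes to the bunker and the Generator is active.
; BunkerPower uses a FlipFlop to alternate the light, hiding it first.
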(event `BunkerPower`
  (bind _pointlight (`self.PointLight`))
  (`/Engine/EditorBlueprintResources/StandardMacros.FlipFlop`
    (:`A`
      (`SceneComponent.SetVisibility` _pointlight false false))
    (:`B`
      (`SceneComponent.SetVisibility` _pointlight true false))))

(event `/Game/FirstPersonBP/Blueprints/Interaction_Interface.Interaction`
  (params (Interactor :type "Actor Object Reference"))
  (if (not (`self.Active`))
    (set `self.Active` true)
    (bind (_direction _newtrack_0) (`Timeline|Timeline_0` :!via `PlayFromStart`)
      (:`Update`
        (`SceneComponent.K2_SetRelativeLocation` (`self.ButtonRoot`) (`KismetMathLibrary.MakeVector` 0.0 _newtrack_0) false false)
        ;[1 1 1] Power Switch is set to deliver Power to the Bunker
        (if (`/Game/Props/Infra/Power/BP_PowerSwitch.Bunker` (`self.PowerSwitch`))
          ;[1 1 1] wGenerator iss Activated
          (if (`/Game/Props/Infra/Power/BP_Generator.GeneratorIsActive` (`self.Generator`))
            (`/Game/Props/AdditionalProps/Doors/Master/BP_BunkerDoor.BunkerButton_Pressd` (`self.BunkerDoor`)))))
      (:`Finished`
        (set `self.Active` false)))))

(fn `UserConstructionScript`)