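; Blockout electric fence actor that plays looping-style low-voltage spark audio and particle effects until it is short-circuited.
; BeginPlay spawns an attenuated spark sound at the fence mesh's location and stores the audio component.
; The ShortCircuit event destroys the five particle components in staggered outside-in pairs with short delays, stopping the sound midway, so the fence visibly powers down.
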(event `ShortCircuit`
  (`ActorComponent.K2_DestroyComponent` (`self.ParticleSystem0`))
  (`ActorComponent.K2_DestroyComponent` (`self.ParticleSystem4`))
  (`KismetSystemLibrary.Delay` 0.2)
  (`ActorComponent.K2_DestroyComponent` (`self.ParticleSystem1`))
  (`ActorComponent.K2_DestroyComponent` (`self.ParticleSystem3`))
  (`AudioComponent.Stop` (stale `self.ReceiveBeginPlay` _returnvalue))
  (`KismetSystemLibrary.Delay` 0.2)
  (`ActorComponent.K2_DestroyComponent` (`self.ParticleSystem2`)))

(event `self.ReceiveBeginPlay`
  (bind _returnvalue (`GameplayStatics.SpawnSoundAtLocation` "/Game/Audio/Samples/A_32682_LowVoltageSparks.A_32682_LowVoltageSparks" (`SceneComponent.K2_GetComponentLocation` (`self.StaticMesh`)) (struct) 0.8 1.0 0.0 "/Game/Audio/Attenuation_ElectricFence.Attenuation_ElectricFence" null)))

(fn `UserConstructionScript`)