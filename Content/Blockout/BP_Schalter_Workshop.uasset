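; BP_Schalter_Workshop is a switch that controls every BP_WorkshopLamp in the level when interacted with.
; Interaction plays a timeline that slides the button along Y, with an Active flag blocking retriggers until it finishes.
; The lamp toggle sits on the timeline's Update, so LightOn flips and all lamps switch on every tick of the animation, not once per press.
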(event `/Game/FirstPersonBP/Blueprints/Interaction_Interface.Interaction`
  (params (Interactor :type "Actor Object Reference"))
  (if (not (`self.Active`))
    (set `self.Active` true)
    (bind (_direction _newtrack_0) (`Timeline|Timeline_0` :!via `PlayFromStart`)
      (:`Update`
        (`SceneComponent.K2_SetRelativeLocation` (`self.ButtonRoot`) (`KismetMathLibrary.MakeVector` 0.0 _newtrack_0) false false)
        (if (`self.LightOn`)
          (bind _outactors (`GameplayStatics.GetAllActorsOfClass` "/Game/Props/BP_WorkshopLamp.BP_WorkshopLamp_C"))
          (`/Game/Props/BP_WorkshopLamp.SwitchOutLight` _outactors)
          (set `self.LightOn` false)
          (else
            (bind _outactors_2 (`GameplayStatics.GetAllActorsOfClass` "/Game/Props/BP_WorkshopLamp.BP_WorkshopLamp_C"))
            (`/Game/Props/BP_WorkshopLamp.SwitchOnLight` _outactors_2)
            (set `self.LightOn` true))))
      (:`Finished`
        (set `self.Active` false)))))

(fn `UserConstructionScript`)