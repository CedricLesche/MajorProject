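; Interactable power switch prop that alternates power between the house and the bunker.
; Each Interaction calls BunkerPower and HousePower on the two linked Schalter references, then a FlipFlop sets the House and Bunker flags.
; Paired timelines slide the two Locator components along X, advancing one and reverting the other.
; CurrentlyInUse blocks re-triggering until the revert finishes, a spark sound plays and a short delay passes.
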(event `/Game/FirstPersonBP/Blueprints/Interaction_Interface.Interaction`
  (params (Interactor :type "Actor Object Reference"))
  (bind _locator_02 (`self.Locator_02`))
  (bind _locator_02_2 (`self.Locator_02`))
  (bind _locator_01 (`self.Locator_01`))
  (bind _locator_01_2 (`self.Locator_01`))
  (bind _returnvalue (`SceneComponent.GetRelativeTransform` _locator_01_2))
  (bind _returnvalue_2 (`SceneComponent.GetRelativeTransform` _locator_02))
  (bind _returnvalue_3 (`SceneComponent.GetRelativeTransform` _locator_02_2))
  (bind _returnvalue_4 (`SceneComponent.GetRelativeTransform` _locator_01))
  (if (not (`self.CurrentlyInUse`))
    (`/Game/Blockout/BP_Schalter_Bunker.BunkerPower` (`self.SchalterBunker`))
    (`/Game/Blockout/BP_Schalter_House.HousePower` (`self.SchalterHouse`))
    (set `self.CurrentlyInUse` true)
    (`/Engine/EditorBlueprintResources/StandardMacros.FlipFlop`
      (:`A`
        (set `self.House` true)
        (set `self.Bunker` false)
        (`|ExecutionSequence`
          (:`then_0`
            (bind (_direction _newtrack_0) (`Timeline|Timeline_0` :!via `PlayFromStart`)
              (:`Update`
                (`SceneComponent.K2_SetRelativeLocation` _locator_01 (`KismetMathLibrary.MakeVector` _newtrack_0 (.y (.location _returnvalue_4)) (.z (.location _returnvalue_4))) false false))))
          (:`then_1`
            (bind (_direction_2 _newtrack_0_2) (`Timeline|Revert` :!via `PlayFromStart`)
              (:`Update`
                (`SceneComponent.K2_SetRelativeLocation` _locator_02_2 (`KismetMathLibrary.MakeVector` _newtrack_0_2 (.y (.location _returnvalue_3)) (.z (.location _returnvalue_3))) false false))
              (:`Finished`
                (`GameplayStatics.PlaySoundAtLocation` "/Game/Audio/Samples/ExternalSounds/A_31348_Spark.A_31348_Spark" (0.0 0.0 0.0) (struct) 0.1 7.0 0.0 null null null)
                (`KismetSystemLibrary.Delay` 0.2)
                (set `self.CurrentlyInUse` false))))))
      (:`B`
        (set `self.Bunker` true)
        (set `self.House` false)
        (`|ExecutionSequence`
          (:`then_0`
            (bind (_direction_3 _newtrack_0_3) (`Timeline|Timeline_1` :!via `PlayFromStart`)
              (:`Update`
                (`SceneComponent.K2_SetRelativeLocation` _locator_02 (`KismetMathLibrary.MakeVector` _newtrack_0_3 (.y (.location _returnvalue_2)) (.z (.location _returnvalue_2))) false false))))
          (:`then_1`
            (bind (_direction_4 _newtrack_0_4) (`Timeline|Revert_2` :!via `PlayFromStart`)
              (:`Update`
                (`SceneComponent.K2_SetRelativeLocation` _locator_01_2 (`KismetMathLibrary.MakeVector` _newtrack_0_4 (.y (.location _returnvalue)) (.z (.location _returnvalue))) false false))
              (:`Finished`
                (`GameplayStatics.PlaySoundAtLocation` "/Game/Audio/Samples/ExternalSounds/A_31348_Spark.A_31348_Spark" (0.0 0.0 0.0) (struct) 0.1 7.0 0.0 null null null)
                (`KismetSystemLibrary.Delay` 0.2)
                (set `self.CurrentlyInUse` false)))))))))

(fn `UserConstructionScript`)