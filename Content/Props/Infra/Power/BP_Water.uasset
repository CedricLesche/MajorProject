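; BP_Water is a water prop that rises and short-circuits the power connector boxes when its DrippingWater event is called.
; Two chained timelines animate the Water component's relative height.
; In parallel, a delayed branch briefly activates a particle effect and calls ShortCircuite on BP_ConectorBox actors found through GetAllActorsOfClass.
; The Activated flag is set afterward so the short circuit does not repeat on later calls.
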(event `DrippingWater`
  (`|ExecutionSequence`
    (:`then_0`
      (`KismetSystemLibrary.Delay` 0.2)
      (bind (_direction _watergetup) (`Timeline|Timeline_0`)
        (:`Update`
          (`SceneComponent.K2_SetRelativeLocation` (`self.Water`) (`KismetMathLibrary.MakeVector` 0.0 0.0 _watergetup) false false))
        (:`Finished`
          (bind (_direction_2 _newtrack_0) (`Timeline|Timeline_1`)
            (:`Update`
              (`SceneComponent.K2_SetRelativeLocation` (`self.Water`) (`KismetMathLibrary.MakeVector` 0.0 0.0 _newtrack_0) false false))))))
    (:`then_1`
      (`KismetSystemLibrary.Delay` 2.0)
      (if (not (`self.activated`))
        (`ActorComponent.Activate` (`self.ParticleSystem`) false)
        (`KismetSystemLibrary.Delay` 0.3)
        (bind _outactors (`GameplayStatics.GetAllActorsOfClass` "/Game/Props/Infra/Power/BP_ConectorBox.BP_ConectorBox_C"))
        (`/Game/Props/Infra/Power/BP_ConectorBox.ShortCircuite` _outactors)
        (`KismetSystemLibrary.Delay` 0.1)
        (`ActorComponent.Deactivate` (`self.ParticleSystem`))
        (set `self.activated` true)))))

(fn `UserConstructionScript`)