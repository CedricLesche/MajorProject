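; BP_Schalter_Workshop is an interactable workshop switch that turns every BP_WorkshopLamp in the level on or off.
; Interaction starts a timeline that slides the Root along Y and plays a switch sound, with an Active flag blocking re-triggers until the animation finishes.
; After a short delay it finds the lamps with GetAllActorsOfClass and toggles them based on its own LightOn state.
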(event `/Game/FirstPersonBP/Blueprints/Interaction_Interface.Interaction`
  (params (Interactor :type "Actor Object Reference"))
  (if (not (`self.Active`))
    (set `self.Active` true)
    (`|ExecutionSequence`
      (:`then_0`
        (bind (_direction _newtrack_0) (`Timeline|Timeline_0` :!via `PlayFromStart`)
          (:`Update`
            (`SceneComponent.K2_SetRelativeLocation` (`self.Root`) (`KismetMathLibrary.MakeVector` 0.0 _newtrack_0) false false))
          (:`Finished`
            (set `self.Active` false))))
      (:`then_1`
        (`GameplayStatics.PlaySoundAtLocation` "/Game/Audio/Samples/OwnSounds/A_Switch.A_Switch" (`SceneComponent.K2_GetComponentLocation` (`self.Root`)) (struct) 0.05 1.0 0.0 "/Game/Audio/ATT_150_1000.ATT_150_1000" null null))
      (:`then_2`
        (`KismetSystemLibrary.Delay` 0.2)
        (if (`self.LightOn`)
          (bind _outactors (`GameplayStatics.GetAllActorsOfClass` "/Game/Props/Infra/Power/BP_WorkshopLamp.BP_WorkshopLamp_C"))
          (`/Game/Props/Infra/Power/BP_WorkshopLamp.SwitchOutLight` _outactors)
          (set `self.LightOn` false)
          (else
            (bind _outactors_2 (`GameplayStatics.GetAllActorsOfClass` "/Game/Props/Infra/Power/BP_WorkshopLamp.BP_WorkshopLamp_C"))
            (`/Game/Props/Infra/Power/BP_WorkshopLamp.SwitchOnLight` _outactors_2)
            (set `self.LightOn` true)))))))

(fn `UserConstructionScript`)