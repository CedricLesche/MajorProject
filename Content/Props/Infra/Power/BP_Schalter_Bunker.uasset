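; Bunker switch prop that plays a click sound and triggers the linked BunkerDoor when interacted with.
; A timeline moves Root along Y and calls BunkerButtonPressd on every update, with an Active flag blocking re-triggering until it finishes.
; BunkerPower flip-flops the point light's visibility, starting with off.
; The power switch and generator checks are disconnected, so the door call is not gated by power.
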(event `BunkerPower`
  (bind _pointlight (`self.PointLight`))
  (`/Engine/EditorBlueprintResources/StandardMacros.FlipFlop`
    (:`A`
      (`SceneComponent.SetVisibility` _pointlight false false))
    (:`B`
      (`SceneComponent.SetVisibility` _pointlight true false))))

(event `/Game/FirstPersonBP/Blueprints/Interaction_Interface.Interaction`
  (params (Interactor :type "Actor Object Reference"))
  (if (not (`self.Active`))
    (set `self.Active` true)
    (`GameplayStatics.PlaySoundAtLocation` "/Game/Audio/Samples/OwnSounds/A_Switch.A_Switch" (`SceneComponent.K2_GetComponentLocation` (`self.Button`)) (struct) 1.0 1.0 0.0 "/Game/Audio/ATT_150_1000.ATT_150_1000" null null)
    (bind (_direction _newtrack_0) (`Timeline|Timeline_0` :!via `PlayFromStart`)
      (:`Update`
        (`SceneComponent.K2_SetRelativeLocation` (`self.Root`) (`KismetMathLibrary.MakeVector` 0.0 _newtrack_0) false false)
        (`/Game/Props/AdditionalProps/Doors/Master/BP_BunkerDoor.BunkerButton_Pressd` (`self.BunkerDoor`)))
      (:`Finished`
        (set `self.Active` false)))))

(fn `UserConstructionScript`)