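; Master Blueprint for a water tank prop with an interactable valve that starts and stops water flow.
; Each interaction toggles the valve, playing or reversing a timeline that rotates the hose handle mesh.
; Opening activates the particle effect and a looping one-second timer that decrements stored water, while closing pauses the timer and deactivates particles.
; When stored water runs out, the flow stops and the tank is flagged empty.
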(event `/Game/FirstPersonBP/Blueprints/Interaction_Interface.Interaction`
  (params (Interactor :type "Actor Object Reference"))
  (if (not (`self.Interaction_Active`))
    (set `self.Interaction_Active` true)
    (if (`self.Ventil_Closed`)
      (set `self.Ventil_Closed` false)
      (`|ExecutionSequence`
        (:`then_0`
          (bind (_direction _newtrack_0) (`Timeline|Timeline_0` :!via `PlayFromStart` :!label _label)
            (:`Update`
              (`SceneComponent.K2_SetRelativeRotation` (`self.SM_Hose_Handle`) (`KismetMathLibrary.MakeRotator` 0.0 0.0 _newtrack_0) false false)
              (set `self.Interaction_Active` false))))
        (:`then_1`
          (`self.Flow Water`)))
      (else
        (set `self.Ventil_Closed` true)
        (`KismetSystemLibrary.K2_PauseTimer` null "Water")
        (`|ExecutionSequence`
          (:`then_0`
            (goto _label :!via `ReverseFromEnd`))
          (:`then_1`
            (`self.End Flow`)))))))

(event `Flow Water`
  (`KismetSystemLibrary.K2_UnPauseTimerHandle` (struct))
  (`KismetSystemLibrary.K2_SetTimer` null "Water" 1.0 true)
  (`ActorComponent.Activate` (`self.ParticleSystem`) false))

(event `End Flow`
  (`KismetSystemLibrary.K2_PauseTimerHandle` (struct))
  (`ActorComponent.Deactivate` (`self.ParticleSystem`)))

(fn `UserConstructionScript`)

(fn `Water`
  (bind _result (`/Engine/EditorBlueprintResources/StandardMacros.DecrementInt` (`self.Water_Stored`))
    (:`  `
      (set `self.Water_Stored` _result)
      (if (<= (`self.Water_Stored`) 0)
        (`KismetSystemLibrary.K2_PauseTimer` null "Water")
        (`self.End Flow`)
        (set `self.Water_Empty` true)))))