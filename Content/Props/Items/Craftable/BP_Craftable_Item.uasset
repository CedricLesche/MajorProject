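; Craftable item prop that, on interaction, turns ingredients from the player's inventory into a product.
; It checks the player InventoryComponent's CollectedItemsMap for three configurable item and quantity requirements, then consumes the first two; the third is only checked.
; The product is registered in the map if absent and collected through the component.
; When requirements are unmet, it reports an error code to FirstPersonGameMode.
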(event `/Game/FirstPersonBP/Blueprints/Interaction_Interface.Interaction`
  (params (Interactor :type "Actor Object Reference"))
  (bind _asfirst_person_character (cast `/Game/FirstPersonBP/Blueprints/FirstPersonCharacter` (`GameplayStatics.GetPlayerCharacter` 0)))
  (bind _inventory_component (`/Game/FirstPersonBP/Blueprints/FirstPersonCharacter.Inventory_Component` _asfirst_person_character))
  (bind _collecteditems_map (`/Game/FirstPersonBP/Blueprints/Inventory_Component.CollectedItems_Map` _inventory_component))
  (if (and (>= (`BlueprintMapLibrary.Map_Find` _collecteditems_map (`self.ItemNeeded_01`)) (`self.Item_01_QuantityNeeded`)) (>= (`BlueprintMapLibrary.Map_Find` _collecteditems_map (`self.ItemNeeded_02`)) (`self.Item_02_QuantityNeeded`)) (>= (`BlueprintMapLibrary.Map_Find` _collecteditems_map (`self.ItemNeeded_03`)) (`self.Item_03_QuantityNeeded`)))
    (`/Game/FirstPersonBP/Blueprints/Inventory_Component.UsedAnItem` _inventory_component (`self.ItemNeeded_01`) (`self.Item_01_QuantityNeeded`))
    (`/Game/FirstPersonBP/Blueprints/Inventory_Component.UsedAnItem` _inventory_component (`self.ItemNeeded_02`) (`self.Item_02_QuantityNeeded`))
    (bind _collecteditems_map_2 (`/Game/FirstPersonBP/Blueprints/Inventory_Component.CollectedItems_Map` _inventory_component))
    (if (not (`BlueprintMapLibrary.Map_Contains` _collecteditems_map_2 (`self.ProductName`)))
      (`BlueprintMapLibrary.Map_Add` _collecteditems_map_2 (`self.ProductName`)))
    (`/Game/FirstPersonBP/Blueprints/Inventory_Component.CollectedAnItem` _inventory_component (`self.ProductName`))
    (else
      (bind _asfirst_person_game_mode (cast `/Game/FirstPersonBP/Blueprints/FirstPersonGameMode` (`GameplayStatics.GetGameMode`)))
      (`/Game/FirstPersonBP/Blueprints/FirstPersonGameMode.UsingObjectError` _asfirst_person_game_mode (`self.ErrorCode`) 0))))

(fn `UserConstructionScript`)