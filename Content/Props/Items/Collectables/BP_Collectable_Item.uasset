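; BP_Collectable_Item is a collectable prop that the player picks up through its Interaction event, guarded by an Active flag so it fires once.
; It ensures ItemName has an entry in the third-person character's InventoryComponent map, starting at zero, then reports the pickup via CollectedAnItem.
; The item hides itself, plays an attenuated collection sound at its location, and destroys itself after a short delay.
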(event `/Game/FirstPersonBP/Blueprints/Interaction_Interface.Interaction`
  (params (Interactor :type "Actor Object Reference"))
  (if (`self.active`)
    (set `self.active` false)
    (bind _asthird_person_character (cast `/Game/FirstPersonBP/Blueprints/ThirdPersonCharacter` (`GameplayStatics.GetPlayerCharacter` 0)))
    (bind _inventory_component (`/Game/FirstPersonBP/Blueprints/ThirdPersonCharacter.Inventory_Component` _asthird_person_character))
    (bind _collecteditems_map (`/Game/FirstPersonBP/Blueprints/Inventory_Component.CollectedItems_Map` _inventory_component))
    (if (not (`BlueprintMapLibrary.Map_Contains` _collecteditems_map (`self.ItemName`)))
      (`BlueprintMapLibrary.Map_Add` _collecteditems_map (`self.ItemName`)))
    (`SceneComponent.SetVisibility` (`self.DefaultSceneRoot`) false true)
    (`/Game/FirstPersonBP/Blueprints/Inventory_Component.CollectedAnItem` _inventory_component (`self.ItemName`))
    (`GameplayStatics.PlaySoundAtLocation` "/Game/Audio/Samples/OwnSounds/A_Collecting.A_Collecting" (`SceneComponent.K2_GetComponentLocation` (`self.CollectableItem`)) (struct) 1.0 1.0 0.0 "/Game/Audio/ATT_150_1000.ATT_150_1000" null null)
    (`KismetSystemLibrary.Delay` 2.0)
    (`self.K2_DestroyActor`)))

(fn `UserConstructionScript`)