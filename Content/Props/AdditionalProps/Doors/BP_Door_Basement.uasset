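; Basement door prop that opens on interaction only from the basement side but can be closed from either side.
; A Box overlap, with no actor filter, sets the PlayerIsInBasement flag, and attempts to open from outside play a fail sound.
; Timelines roll a Scene component, then swing the Root's yaw after a short delay, with Close played in reverse to shut.
; AnimationInProgress blocks re-triggering during motion or the fail cooldown.
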(event `/Game/FirstPersonBP/Blueprints/Interaction_Interface.Interaction`
  (params (Interactor :type "Actor Object Reference"))
  (if (not (`self.AnimationInProgress`))
    (set `self.AnimationInProgress` true)
    (if (`self.Player is in Basement`)
      (if (`self.Door_Closed`)
        (`GameplayStatics.PlaySoundAtLocation` "/Game/Audio/Samples/OwnSounds/A_Door_Open.A_Door_Open" (`SceneComponent.K2_GetComponentLocation` (`self.Root`)) (struct) 1.0 1.0 0.0 null null null)
        (`|ExecutionSequence`
          (:`then_0`
            (bind (_direction _newtrack_0) (`Timeline|Timeline_0` :!via `PlayFromStart`)
              (:`Update`
                (`SceneComponent.K2_SetRelativeRotation` (`self.Scene`) (`KismetMathLibrary.MakeRotator` _newtrack_0) false false))))
          (:`then_1`
            (`KismetSystemLibrary.Delay` 0.2)
            (bind (_direction_2 _doorrotation) (`Timeline|Open` :!via `PlayFromStart`)
              (:`Update`
                (`SceneComponent.K2_SetRelativeLocationAndRotation` (`self.Root`) (0.0 0.0 0.0) (`KismetMathLibrary.MakeRotator` 0.0 0.0 _doorrotation) false false)
                (set `self.Door_Closed` false))
              (:`Finished`
                (set `self.AnimationInProgress` false)))))
        (else
          (bind (_direction_3 _doorrotation_2) (`Timeline|Close` :!via `ReverseFromEnd` :!label _label)
            (:`Update`
              (`SceneComponent.K2_SetRelativeLocationAndRotation` (`self.Root`) (0.0 0.0 0.0) (`KismetMathLibrary.MakeRotator` 0.0 0.0 _doorrotation_2) false false)
              (set `self.Door_Closed` true))
            (:`Finished`
              (`GameplayStatics.PlaySoundAtLocation` "/Game/Audio/Samples/OwnSounds/A_HeavyDoor_Close.A_HeavyDoor_Close" (`SceneComponent.K2_GetComponentLocation` (`self.Root`)) (struct) 1.0 1.0 0.0 null null null)
              (set `self.AnimationInProgress` false)))))
      (elif (`self.Door_Closed`)
        (`GameplayStatics.PlaySoundAtLocation` "/Game/Audio/Samples/OwnSounds/A_HeavyDoor_Fail.A_HeavyDoor_Fail" (`SceneComponent.K2_GetComponentLocation` (`self.Root`)) (struct) 1.0 0.8 0.0 null null null)
        (`KismetSystemLibrary.Delay` 1.0)
        (set `self.AnimationInProgress` false)
        (else
          (goto _label :!via `ReverseFromEnd`))))))

(event `self.Box.OnComponentBeginOverlap`
  (params (OverlappedComponent :type "PrimitiveComponent Object Reference") (OtherActor :type "Actor Object Reference") (OtherComp :type "PrimitiveComponent Object Reference") (OtherBodyIndex :type Integer) (bFromSweep :type Boolean) (SweepResult :type "HitResult Structure (by ref)"))
  ;[1 1 1] Is Player in Basement?
  (set `self.Player is in Basement` true))

(event `self.Box.OnComponentEndOverlap`
  (params (OverlappedComponent :type "PrimitiveComponent Object Reference") (OtherActor :type "Actor Object Reference") (OtherComp :type "PrimitiveComponent Object Reference") (OtherBodyIndex :type Integer))
  ;[1 1 1] Is Player in Basement?
  (set `self.Player is in Basement` false))

(fn `UserConstructionScript`)