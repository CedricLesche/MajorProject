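; BP_PowerFence_Door is an electrified fence door that only swings once its power is cut.
; ShortCircuit_Door waits briefly, hides four particle systems and sets PowerDeactivated.
; Interaction plays a spark sound while powered, otherwise runs the Open or reversed Close timeline to yaw the root, with door sounds.
; An AnimationInProgress flag blocks re-triggering, and the DoorOpen flag reads inverted: true selects the Open timeline, which sets it false.
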(event `Short Circuit_Door`
  ;[1 1 1] Clear Particle
  (`KismetSystemLibrary.Delay` 0.3)
  (`SceneComponent.SetVisibility` (`self.ParticleSystem2`) false true)
  (`SceneComponent.SetVisibility` (`self.ParticleSystem3`) false true)
  (`SceneComponent.SetVisibility` (`self.ParticleSystem0`) false true)
  (`SceneComponent.SetVisibility` (`self.ParticleSystem1`) false true)
  (set `self.PowerDeactivated` true))

(event `/Game/FirstPersonBP/Blueprints/Interaction_Interface.Interaction`
  (params (Interactor :type "Actor Object Reference"))
  (bind _returnvalue (`SceneComponent.K2_GetComponentLocation` (`self.Root`)))
  (if (`self.PowerDeactivated`)
    (if (not (`self.AnimationInProgress`))
      (set `self.AnimationInProgress` true)
      (if (`self.Door_Open`)
        (`GameplayStatics.PlaySoundAtLocation` "/Game/Audio/Samples/OwnSounds/A_Door_Open.A_Door_Open" _returnvalue (struct) 1.0 1.0 0.0 "/Game/Audio/ATT_800_1500.ATT_800_1500" null null)
        (bind (_direction _doorrotation) (`Timeline|Open` :!via `PlayFromStart`)
          (:`Update`
            (`SceneComponent.K2_SetRelativeLocationAndRotation` (`self.Root`) (0.0 0.0 0.0) (`KismetMathLibrary.MakeRotator` 0.0 0.0 _doorrotation) false false)
            (set `self.Door_Open` false))
          (:`Finished`
            (set `self.AnimationInProgress` false)))
        (else
          (bind (_direction_2 _doorrotation_2) (`Timeline|Close` :!via `ReverseFromEnd`)
            (:`Update`
              (`SceneComponent.K2_SetRelativeLocationAndRotation` (`self.Root`) (0.0 0.0 0.0) (`KismetMathLibrary.MakeRotator` 0.0 0.0 _doorrotation_2) false false)
              (set `self.Door_Open` true))
            (:`Finished`
              (`GameplayStatics.PlaySoundAtLocation` "/Game/Audio/Samples/OwnSounds/A_HeavyDoor_Close.A_HeavyDoor_Close" _returnvalue (struct) 1.0 1.0 0.0 "/Game/Audio/ATT_800_1500.ATT_800_1500" null null)
              (set `self.AnimationInProgress` false))))))
    (else
      (`GameplayStatics.PlaySoundAtLocation` "/Game/Audio/Samples/ExternalSounds/A_31348_Spark.A_31348_Spark" (`SceneComponent.K2_GetComponentLocation` (`self.Root`)) (struct) 1.5 0.8 0.0 "/Game/Audio/ATT_150_1000.ATT_150_1000" null null))))

(fn `UserConstructionScript`)