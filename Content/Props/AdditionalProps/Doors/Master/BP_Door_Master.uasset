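; Master door Blueprint that players open and close through an Interaction event, gated by an item cost from their inventory.
; The cost is paid on every toggle or only on first opening, depending on CostsEveryTime, and a failed check plays a sound.
; Payment can redden and hide a destroyable mesh before timelines animate the handle and swing the door, with AnimationInProgress blocking re-triggers.
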(event `/Game/FirstPersonBP/Blueprints/Interaction_Interface.Interaction`
  (params (Interactor :type "Actor Object Reference"))
  (bind _destroyablemesh (`self.DestroyableMesh`))
  (bind _asthird_person_character (cast `/Game/FirstPersonBP/Blueprints/ThirdPersonCharacter` (`GameplayStatics.GetPlayerCharacter` 0)))
  (if (`self.CostsEveryTime`)
    (bind _inventory_component (`/Game/FirstPersonBP/Blueprints/ThirdPersonCharacter.Inventory_Component` _asthird_person_character))
    (bind _value (`BlueprintMapLibrary.Map_Find` (`/Game/FirstPersonBP/Blueprints/Inventory_Component.CollectedItems_Map` _inventory_component) (`self.ItemNeededToOpen`)))
    (if (>= _value 1) :!label _label
      (if (>= _value (`self.ItemCost`))
        (if (not (`self.AnimationInProgress`))
          (set `self.AnimationInProgress` true)
          (`/Game/FirstPersonBP/Blueprints/Inventory_Component.UsedAnItem` _inventory_component (`self.ItemNeededToOpen`) (`self.ItemCost`))
          (if (`self.DestroyableObject`)
            (`PrimitiveComponent.SetMaterial` _destroyablemesh 0 "/Game/MAterials/Childs/MI_Base_Red.MI_Base_Red")
            (`KismetSystemLibrary.Delay` 0.5)
            (`SceneComponent.SetVisibility` _destroyablemesh false true)
            (`KismetSystemLibrary.Delay` 1.0))
          (set `self.OpendOnce` true)
          (if (`self.Door_Closed`) :!label _label_2
            (`|ExecutionSequence`
              (:`then_0`
                (bind (_direction _newtrack_0) (`Timeline|Timeline_2` :!via `PlayFromStart`)
                  (:`Update`
                    (`SceneComponent.K2_SetRelativeRotation` (`self.HandleGRP`) (`KismetMathLibrary.MakeRotator` _newtrack_0) false false))))
              (:`then_1`
                (`KismetSystemLibrary.Delay` 0.2)
                (bind (_direction_2 _doorrotation) (`Timeline|Timeline_0` :!via `PlayFromStart`)
                  (:`Update`
                    (`SceneComponent.K2_SetRelativeLocationAndRotation` (`self.BladeRoot`) (0.0 0.0 0.0) (`KismetMathLibrary.MakeRotator` 0.0 0.0 _doorrotation) false false)
                    (set `self.Door_Closed` false))
                  (:`Finished`
                    (`GameplayStatics.PlaySoundAtLocation` (`self.OpenSound`) (`SceneComponent.K2_GetComponentLocation` (`self.BladeRoot`)) (struct) 1.0 1.0 0.0 "/Game/Audio/Attenuation_Grashopper.Attenuation_Grashopper" null null)
                    (set `self.AnimationInProgress` false)))))
            (else
              (bind (_direction_3 _doorrotation_2) (`Timeline|Timeline_1` :!via `ReverseFromEnd`)
                (:`Update`
                  (`SceneComponent.K2_SetRelativeLocationAndRotation` (`self.BladeRoot`) (0.0 0.0 0.0) (`KismetMathLibrary.MakeRotator` 0.0 0.0 _doorrotation_2) false false)
                  (set `self.Door_Closed` true))
                (:`Finished`
                  (`GameplayStatics.PlaySoundAtLocation` (`self.Close_Sound`) (`SceneComponent.K2_GetComponentLocation` (`self.BladeRoot`)) (struct) 1.0 1.0 0.0 null null null)
                  (set `self.AnimationInProgress` false))))))
        (else
          (`GameplayStatics.PlaySoundAtLocation` (`self.FailSound`) (`SceneComponent.K2_GetComponentLocation` (`self.BladeRoot`)) (struct) 1.0 1.0 0.0 null null null :!label _label_3)))
      (else
        (goto _label_3)))
    (elif (`self.OpendOnce`)
      (if (not (`self.AnimationInProgress`))
        (set `self.AnimationInProgress` true)
        (goto _label_2))
      (else
        (goto _label)))))

(fn `UserConstructionScript`)