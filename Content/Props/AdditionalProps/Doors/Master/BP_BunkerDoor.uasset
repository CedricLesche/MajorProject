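; Bunker door prop that serves as the game's ending trigger when its button event fires.
; A timeline swings the door's root around yaw while the player camera fades out and holds.
; After timed delays it disables character movement, then adds the EndScreen widget, shows the mouse cursor and switches input to UI only.
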(event `BunkerButton_Pressd`
  (bind _returnvalue (`GameplayStatics.GetPlayerController` 0))
  (`|ExecutionSequence`
    (:`then_0`
      (bind (_direction _newtrack_0) (`Timeline|Timeline_0` :!via `PlayFromStart`)
        (:`Update`
          (`SceneComponent.K2_SetRelativeLocationAndRotation` (`self.Root`) (0.0 0.0 0.0) (`KismetMathLibrary.MakeRotator` 0.0 0.0 _newtrack_0) false false))))
    (:`then_1`
      (`PlayerCameraManager.StartCameraFade` :`self` (`GameplayStatics.GetPlayerCameraManager` 0) :`ToAlpha` 1.0 :`Duration` 5.0 :`bHoldWhenFinished` true)
      (`KismetSystemLibrary.Delay` 5.0)
      (`CharacterMovementComponent.DisableMovement` (`Character.CharacterMovement` (`GameplayStatics.GetPlayerCharacter` 0)))
      (`KismetSystemLibrary.Delay` 2.5)
      (bind _returnvalue_2 (`|CreateWidget` "/Game/UI/EndScreen.EndScreen_C"))
      (`UserWidget.AddToViewport` _returnvalue_2 0)
      (set `PlayerController.bShowMouseCursor` true _returnvalue)
      (`WidgetBlueprintLibrary.SetInputMode_UIOnlyEx` _returnvalue _returnvalue_2))))

(fn `UserConstructionScript`)