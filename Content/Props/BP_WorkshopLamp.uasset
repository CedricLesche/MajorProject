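; Workshop lamp prop whose point light is turned on and off through the SwitchOnLight and SwitchOutLight events.
; Switching on shows the light and plays a timeline that drives its intensity, then a second flicker timeline takes over intensity if CanFlicker is set.
; Switching off only hides the light, without stopping either timeline.
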(event `SwitchOnLight`
  (`SceneComponent.SetVisibility` (`self.PointLight`) true false)
  (bind (_direction _newtrack_0) (`Timeline|Timeline_1`)
    (:`Update`
      (`LightComponent.SetIntensity` (`self.PointLight`) _newtrack_0))
    (:`Finished`
      (if (`self.CanFlicker`)
        (bind (_direction_2 _newtrack_0_2) (`Timeline|Timeline_0`)
          (:`Update`
            (`LightComponent.SetIntensity` (`self.PointLight`) _newtrack_0_2)))))))

(event `SwitchOutLight`
  (`SceneComponent.SetVisibility` (`self.PointLight`) false false))

(fn `UserConstructionScript`)